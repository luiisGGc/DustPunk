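; CAR is a physics-driven vehicle Blueprint using raycast suspension on a Box body.
; Each tick, four wheel points trace downward and push the Box along the trace, harder as the ground gets closer, with no damping.
; A constant mass-scaled forward force is also applied every tick.
; Enhanced Input ramps Aceleracion while accelerating and zeroes it on release, but that value does not feed the drive force.
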(event Input|EnhancedActionEvents|EnhancedInputActionIA_Acelerar
  (params (ActionValue :type Float%20%28double-precision%29) (ElapsedSeconds :type Float%20%28double-precision%29) (TriggeredSeconds :type Float%20%28double-precision%29) (InputAction :type Input%20Action%20Object%20Reference :default "/Game/Inputs/IA_Acelerar.IA_Acelerar"))
  (:Triggered
    (Variables|Default|SetAceleracion (Math|Interpolation|FInterpTo (Variables|Default|GetAceleracion) 1.0 (Utilities|Time|GetWorldDeltaSeconds) 0.5)))
  (:Completed
    (Variables|Default|SetAceleracion 0.0)))

(event EventTick
  (params (DeltaSeconds :type Float%20%28single-precision%29))
  (CallFunction|SuspensionCAST (Variables|Default|GetDI))
  (CallFunction|SuspensionCAST (Variables|Default|GetDD))
  (CallFunction|SuspensionCAST (Variables|Default|GetScene))
  (CallFunction|SuspensionCAST (Variables|Default|GetScene1))
  (Physics|AddForce (Variables|Default|GetBox) (* (Math|Vector|GetForwardVector (Variables|Default|GetBox)) 1e+04 (Physics|GetMass (Variables|Default|GetBox))) "None" false))

(event EventBeginPlay
  (Input|AddMappingContext (PlayerController|LocalPlayerSubsystems|GetEnhancedInputLocalPlayerSubsystem (Game|GetPlayerController 0)) "/Game/Inputs/IC_Carro.IC_Carro" 0 "(bIgnoreAllPressedKeysUntilRelease=True,bForceImmediately=False,bNotifyUserSettings=False)"))

(fn ConstructionScript)

(fn SuspensionCAST
  (params (WheelComp :type Scene%20Component%20Object%20Reference))
  (bind _returnvalue (Transformation|GetWorldLocation WheelComp))
  (bind _outhit (Collision|LineTraceByChannel _returnvalue (+ _returnvalue (* (Math|Vector|GetUpVector WheelComp) -6e+01)) "TraceTypeQuery1" false 0 "ForOneFrame"))
  (if (.bBlockingHit (Collision|BreakHitResult _outhit))
    (Class|PrimitiveComponent|AddForceatLocation (Variables|Default|GetBox) (* (Math|Vector|GetUnitDirection(Vector) (.TraceEnd (Collision|BreakHitResult _outhit)) (.TraceStart (Collision|BreakHitResult _outhit))) (- 1.0 (Math|Float|NormalizetoRange (.Distance (Collision|BreakHitResult _outhit)) 0.0 6e+01)) 9e+04) (Transformation|GetWorldLocation WheelComp) "None")))