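; Enemy car Blueprint that chases the first Carro actor when it comes within detection range.
; Each tick, SuspensionCAST traces down from four wheel points and pushes the physics Box up at each hit, scaled by compression.
; Chasing applies a mass-scaled force toward the target and smoothly rotates the car to face it.
; Constant local downforce, plus extra world-down acceleration while chasing, presses the car downward.
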(event EventTick
  (params (DeltaSeconds :type Float%20%28single-precision%29))
  (bind _self self)
  (bind _box (Variables|Default|GetBox))
  (bind _box_2 (Variables|Default|GetBox))
  (bind _returnvalue (Transformation|GetActorLocation _self))
  (Utilities|FlowControl|Sequence
    (:then_0
      (CallFunction|SuspensionCAST (Variables|Default|GetDI))
      (CallFunction|SuspensionCAST (Variables|Default|GetDD))
      (CallFunction|SuspensionCAST (Variables|Default|GetScene))
      (CallFunction|SuspensionCAST (Variables|Default|GetScene1))
      (bind _outactors (Actor|GetAllActorsOfClass "/Game/BluePrints/Carro.Carro_C"))
      (Utilities|IsValid (Utilities|Array|Get(acopy) _outactors)
        (:Is%20Valid
          (if (< (Math|Vector|VectorLength (- (Transformation|GetActorLocation (Utilities|Array|Get(acopy) _outactors)) _returnvalue)) (Variables|Default|GetDistanciaDeteccion))
            (Physics|AddForce _box_2 (* (* (Math|Vector|Normalize (- (Transformation|GetActorLocation (Utilities|Array|Get(acopy) _outactors)) _returnvalue)) (Variables|Default|GetVelocidadPersecucion)) (Physics|GetMass _box_2)) "None" false)
            (Physics|AddForce (Variables|Default|GetBox) "0.000000,0.000000,-5000.000000" "None" true)
            (Transformation|SetActorRotation _self (Math|Interpolation|RInterpTo (Transformation|GetActorRotation _self) (Math|Rotator|FindLookatRotation _returnvalue (Transformation|GetActorLocation (Utilities|Array|Get(acopy) _outactors))) (Utilities|Time|GetWorldDeltaSeconds) 2.0))))))
    (:then_1
      (Physics|AddForce _box (* (* (* (Transformation|GetActorUpVector self) -1.0) 5e+03) (Physics|GetMass _box)) "None" false))))

(fn ConstructionScript)

(fn SuspensionCAST
  (params (WheelComp :type Scene%20Component%20Object%20Reference))
  (bind _returnvalue (Transformation|GetWorldLocation WheelComp))
  (bind _outhit (Collision|LineTraceByChannel _returnvalue (+ _returnvalue (* (Math|Vector|GetUpVector WheelComp) -6e+01)) (Utilities|Enum|LiteralenumETraceTypeQuery "TraceTypeQuery1") false (Utilities|Array|MakeArray 0) (Utilities|Enum|LiteralenumEDrawDebugTrace "ForOneFrame")))
  (if (.bBlockingHit (Collision|BreakHitResult _outhit))
    (Class|PrimitiveComponent|AddForceatLocation (Variables|Default|GetBox) (* (* (Math|Vector|GetUnitDirection(Vector) (.TraceEnd (Collision|BreakHitResult _outhit)) (.TraceStart (Collision|BreakHitResult _outhit))) (- 1.0 (Math|Float|NormalizetoRange (.Distance (Collision|BreakHitResult _outhit)) 0.0 6e+01))) 9e+04) _returnvalue "None")))